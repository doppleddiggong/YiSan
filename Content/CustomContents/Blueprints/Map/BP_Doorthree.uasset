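; BP_Doorthree is a double-door Blueprint that swings its left and right doors open or closed through two animation events.
; Each event saves the current rotations as start points, stops the opposite timeline and plays its own from the start.
; The timeline alpha drives DoorLerp, an eased rotator lerp toward per-door open rotations or a shared closed rotation.
; Starting from current rotations lets a reversal mid-swing continue without snapping.
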(event EventPlayOpenDoorAnimation
  ;[0.15 0.1302 0 0.5] OpenAnimation
  (CallFunction|SaveStartRot)
  (Audio|Components|Audio|Stop (Variables|Default|GetCloseAnim))
  (bind _openclose (Timeline|OpenAnim PlayFromStart)
    (:Update
      (Utilities|FlowControl|Sequence
        (:then_0
          (CallFunction|DoorLerp (Variables|Default|GetDoor_Right) (Variables|Temp|GetR_Start) (Variables|Default|GetR_Open) _openclose "Linear"))
        (:then_1
          (CallFunction|DoorLerp (Variables|Default|GetDoor_Left) (Variables|Temp|GetL_Start) (Variables|Default|GetL_Open) _openclose "Linear"))))))

(event EventPlayCloseDoorAnimation
  ;[0.15 0.0124 0 0.5] CloseAnimation
  (CallFunction|SaveStartRot)
  (Audio|Components|Audio|Stop (Variables|Default|GetOpenAnim))
  (bind _openclose (Timeline|CloseAnim PlayFromStart)
    (:Update
      (Utilities|FlowControl|Sequence
        (:then_0
          (CallFunction|DoorLerp (Variables|Default|GetDoor_Left) (Variables|Temp|GetL_Start) (Variables|Default|GetClose) _openclose "Linear"))
        (:then_1
          (CallFunction|DoorLerp (Variables|Default|GetDoor_Right) (Variables|Temp|GetR_Start) (Variables|Default|GetClose) _openclose "Linear"))))))

(fn ConstructionScript)

(fn DoorLerp
  (params (Target :type Mesh%20Component%20Object%20Reference) (A :type Rotator) (B :type Rotator) (Alpha :type Float%20%28single-precision%29) (EaseType :type EEaseType%20Enum :default "Linear"))
  (Transformation|SetRelativeRotation Target (Class|EaseFunctionLibrary|LerpRotatorEase A B Alpha EaseType) false false))

(fn SaveStartRot
  (Variables|Temp|SetL_Start (Variables|/Script/Engine.SceneComponent|GetRelativeRotation (Variables|Default|GetDoor_Left)))
  (Variables|Temp|SetR_Start (Variables|/Script/Engine.SceneComponent|GetRelativeRotation (Variables|Default|GetDoor_Right))))